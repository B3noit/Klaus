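; BP_BOX is a Blueprint for a numbered box that displays its BoxNumber as text.
; On BeginPlay it converts BoxNumber to text and writes the same value to six TextRender components.
; The construction script is empty, so the labels are only set from BoxNumber when play begins.
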(event `self.ReceiveBeginPlay`
  (bind _returnvalue (`KismetTextLibrary.Conv_StringToText` (`self.BoxNumber`)))
  (`TextRenderComponent.K2_SetText` (`self.TextRender`) _returnvalue)
  (`TextRenderComponent.K2_SetText` (`self.TextRender1`) _returnvalue)
  (`TextRenderComponent.K2_SetText` (`self.TextRender2`) _returnvalue)
  (`TextRenderComponent.K2_SetText` (`self.TextRender3`) _returnvalue)
  (`TextRenderComponent.K2_SetText` (`self.TextRender4`) _returnvalue)
  (`TextRenderComponent.K2_SetText` (`self.TextRender5`) _returnvalue))

(fn `UserConstructionScript`)