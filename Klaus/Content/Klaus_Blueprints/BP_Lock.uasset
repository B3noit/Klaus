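; BP_Lock is a three-slot puzzle lock that reveals a Valid component when the displayed numbers match the solution.
; Each box trigger detects an overlapping BP_BOX and writes its BoxNumber to that slot's text.
; VerifSolution, not called within this graph, compares the text to solution values.
; As written, it checks the second slot twice and never checks the third.
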(event `VerifSolution`
  (if (and (`KismetTextLibrary.EqualEqual_TextText` (`TextRenderComponent.Text` (`self.Lock`)) (`KismetTextLibrary.Conv_StringToText` (`self.LockSolution1`))) (`KismetTextLibrary.EqualEqual_TextText` (`TextRenderComponent.Text` (`self.Lock1`)) (`KismetTextLibrary.Conv_StringToText` (`self.LockSolution2`))) (`KismetTextLibrary.EqualEqual_TextText` (`TextRenderComponent.Text` (`self.Lock1`)) (`KismetTextLibrary.Conv_StringToText` (`self.LockSolution2`))))
    (`SceneComponent.SetVisibility` (`self.valid`) true false)))

(event `self.Box.OnComponentBeginOverlap`
  (params (OverlappedComponent :type "PrimitiveComponent Object Reference") (OtherActor :type "Actor Object Reference") (OtherComp :type "PrimitiveComponent Object Reference") (OtherBodyIndex :type Integer) (bFromSweep :type Boolean) (SweepResult :type "HitResult Structure (by ref)"))
  (bind _asbp_box (cast `/Game/Klaus_Blueprints/BP_BOX` OtherActor))
  (`TextRenderComponent.K2_SetText` (`self.Lock`) (`KismetTextLibrary.Conv_StringToText` (`/Game/Klaus_Blueprints/BP_BOX.BoxNumber` _asbp_box))))

(event `self.Box1.OnComponentBeginOverlap`
  (params (OverlappedComponent :type "PrimitiveComponent Object Reference") (OtherActor :type "Actor Object Reference") (OtherComp :type "PrimitiveComponent Object Reference") (OtherBodyIndex :type Integer) (bFromSweep :type Boolean) (SweepResult :type "HitResult Structure (by ref)"))
  (bind _asbp_box (cast `/Game/Klaus_Blueprints/BP_BOX` OtherActor))
  (`TextRenderComponent.K2_SetText` (`self.Lock1`) (`KismetTextLibrary.Conv_StringToText` (`/Game/Klaus_Blueprints/BP_BOX.BoxNumber` _asbp_box))))

(event `self.Box2.OnComponentBeginOverlap`
  (params (OverlappedComponent :type "PrimitiveComponent Object Reference") (OtherActor :type "Actor Object Reference") (OtherComp :type "PrimitiveComponent Object Reference") (OtherBodyIndex :type Integer) (bFromSweep :type Boolean) (SweepResult :type "HitResult Structure (by ref)"))
  (bind _asbp_box (cast `/Game/Klaus_Blueprints/BP_BOX` OtherActor))
  (`TextRenderComponent.K2_SetText` (`self.Lock2`) (`KismetTextLibrary.Conv_StringToText` (`/Game/Klaus_Blueprints/BP_BOX.BoxNumber` _asbp_box))))

(fn `UserConstructionScript`)